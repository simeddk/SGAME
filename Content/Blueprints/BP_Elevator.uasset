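; Elevator actor that carries the player vertically from its starting position to the height of a Target actor.
; Player overlap turns the emissive green, plays a door sound and runs a slowed timeline that lerps only Z, restoring red on completion.
; Any actor ending overlap stops the timeline in place, with no return movement.
; The construction script makes it movable and creates the dynamic material, initially red.
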(event EventBeginPlay
  (Variables|Default|SetStart (Transformation|GetActorLocation)))

(event Collision|EventActorBeginOverlap
  (params (OtherActor :type Actor%20Object%20Reference))
  (bind _start (Variables|Default|GetStart))
  (bind (_x _y) (Math|Vector|BreakVector _start))
  (Utilities|Casting|CastToBP_Player OtherActor)
  (Rendering|Material|SetVectorParameterValue (Variables|Default|GetDynamicMaterial) "Emissive" "(R=0.000000,G=20.000000,B=0.000000,A=1.000000)" :!class /Script/Engine.MaterialInstanceDynamic)
  (CallFunction|PlaySoundStatic "/Game/Door/Doom-Door-Open_mp3.Doom-Door-Open_mp3" self)
  (Components|Timeline|SetPlayRate (Variables|Default|GetTimeline) 0.25)
  (bind _output (Timeline|Timeline Play)
    (:Update
      (Transformation|SetActorLocation (Math|Vector|Lerp(Vector) _start (Math|Vector|MakeVector _x _y (.Z (Math|Vector|BreakVector (Transformation|GetActorLocation (Variables|Default|GetTarget))))) _output) false false))
    (:Finished
      (Rendering|Material|SetVectorParameterValue (Variables|Default|GetDynamicMaterial) "Emissive" "(R=20.000000,G=0.000000,B=0.000000,A=1.000000)" :!class /Script/Engine.MaterialInstanceDynamic))))

(event Collision|EventActorEndOverlap
  (params (OtherActor :type Actor%20Object%20Reference))
  (bind _start (Variables|Default|GetStart))
  (bind (_x _y) (Math|Vector|BreakVector _start))
  (bind _output (Timeline|Timeline Stop)
    (:Update
      (Transformation|SetActorLocation (Math|Vector|Lerp(Vector) _start (Math|Vector|MakeVector _x _y (.Z (Math|Vector|BreakVector (Transformation|GetActorLocation (Variables|Default|GetTarget))))) _output) false false))
    (:Finished
      (Rendering|Material|SetVectorParameterValue (Variables|Default|GetDynamicMaterial) "Emissive" "(R=20.000000,G=0.000000,B=0.000000,A=1.000000)" :!class /Script/Engine.MaterialInstanceDynamic))))

(fn ConstructionScript
  (Transformation|SetMobility "Movable")
  (bind _returnvalue (Rendering|Material|CreateDynamicMaterialInstance (Rendering|Material|GetMaterial (Variables|Default|GetStaticMesh) 0) "None" :!class /Script/Engine.KismetMaterialLibrary))
  (bind _output_get (Variables|Default|SetDynamicMaterial _returnvalue))
  (Rendering|Material|SetMaterial (Variables|Default|GetStaticMesh) 0 _output_get)
  (Rendering|Material|SetVectorParameterValue (Variables|Default|GetDynamicMaterial) "Emissive" "(R=20.000000,G=0.000000,B=0.000000,A=1.000000)" :!class /Script/Engine.MaterialInstanceDynamic))