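; BP_KillDoor is a door that dissolves away once every actor in its MustKill list is dead.
; Tick checks the list only while the first player character is within CheckDistance.
; When all are dead, a DoOnce starts a timeline that drives the Zoom scalar on a dynamic material created in the construction script, then destroys the door when it finishes.
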(event EventBeginPlay)

(event Collision|EventActorBeginOverlap
  (params (OtherActor :type Actor%20Object%20Reference)))

(event EventTick
  (params (DeltaSeconds :type Float%20%28single-precision%29))
  (Variables|Default|SetbAllDead true)
  (if (<= (Transformation|GetDistanceTo (Game|GetPlayerCharacter 0) self) (Variables|Default|GetCheckDistance))
    (for _array_element (Variables|Default|GetMustKill)
      (Variables|Default|SetbAllDead (and (Default|IsDead _array_element) (Variables|Default|GetbAllDead))))
    (if (Variables|Default|GetbAllDead)
      (Utilities|FlowControl|DoOnce false
        (:Completed
          (bind _out (Timeline|tineline PlayFromStart)
            (:Update
              (Rendering|Material|SetScalarParameterValue (Variables|Default|GetDynamicMAT) "Zoom" _out :!class /Script/Engine.MaterialInstanceDynamic))
            (:Finished
              (Actor|DestroyActor))))))))

(fn ConstructionScript
  (bind _returnvalue (Rendering|Material|CreateDynamicMaterialInstance (Rendering|Material|GetMaterial (Variables|Default|GetMesh) 0) "None" :!class /Script/Engine.KismetMaterialLibrary))
  (bind _output_get (Variables|Default|SetDynamicMAT _returnvalue))
  (Rendering|Material|SetMaterial (Variables|Default|GetMesh) 0 _output_get))