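; BP_TriggerLaser is a trigger actor that notifies a linked TriggerTo object when a Character hits its static mesh.
; On BeginPlay it creates a dynamic material instance for the mesh and sets its Emissive color to red.
; A Character hit calls OnCollision on TriggerTo, if valid, and switches Emissive to a bright blue, with no reset or guard against repeat hits.
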(event OnComponentHit(StaticMesh)
  (params (HitComponent :type Primitive%20Component%20Object%20Reference) (OtherActor :type Actor%20Object%20Reference) (OtherComp :type Primitive%20Component%20Object%20Reference) (NormalImpulse :type Vector :default "0, 0, 0") (Hit :type Hit%20Result%20Structure%20%28by%20ref%29))
  (Utilities|Casting|CastToCharacter OtherActor)
  (bind _triggerto (Variables|Default|GetTriggerTo)
    (:then
      (Default|OnCollision _triggerto)
      (Rendering|Material|SetVectorParameterValue (Variables|Default|GetDynamicMaterial) "Emissive" "(R=0.000000,G=0.000000,B=20.000000,A=1.000000)" :!class /Script/Engine.MaterialInstanceDynamic))
    (:else)))

(event EventBeginPlay
  (bind _returnvalue (Rendering|Material|CreateDynamicMaterialInstance (Rendering|Material|GetMaterial (Variables|Default|GetStaticMesh) 0) "None" :!class /Script/Engine.KismetMaterialLibrary))
  (bind _output_get (Variables|Default|SetDynamicMaterial _returnvalue))
  (Rendering|Material|SetMaterial (Variables|Default|GetStaticMesh) 0 _output_get)
  (Rendering|Material|SetVectorParameterValue (Variables|Default|GetDynamicMaterial) "Emissive" "(R=1.000000,G=0.000000,B=0.000000,A=1.000000)" :!class /Script/Engine.MaterialInstanceDynamic))

(fn ConstructionScript)