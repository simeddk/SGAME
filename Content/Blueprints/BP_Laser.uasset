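; BP_Laser is a laser actor whose static mesh components start hidden and without collision, gathered into an array on BeginPlay.
; OnCollision reveals every mesh with query and physics collision, gated by a DoOnce that the Reset event re-arms.
; OffCollisions hides the meshes and disables their collision again without resetting that gate.
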(event Custom|OnCollision
  (Utilities|FlowControl|DoOnce false
    (:Completed
      (for _array_element (Variables|Default|GetSMS)
        (Development|SetHiddeninGame _array_element false false)
        (Collision|SetCollisionEnabled _array_element "QueryAndPhysics")))))

(event Custom|OffCollisions
  (for _array_element (Variables|Default|GetSMS)
    (Development|SetHiddeninGame _array_element true false)
    (Collision|SetCollisionEnabled _array_element "NoCollision")))

(event Custom|Reset
  (Utilities|FlowControl|DoOnce false) ; enters at Reset
)

(event EventBeginPlay
  (bind _output_get (Variables|Default|SetSMS (Actor|GetComponentsByClass "/Script/Engine.StaticMeshComponent")))
  (for _array_element _output_get
    (Development|SetHiddeninGame _array_element true false)
    (Collision|SetCollisionEnabled _array_element "NoCollision")))

(fn ConstructionScript)