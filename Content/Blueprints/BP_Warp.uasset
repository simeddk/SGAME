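; BP_Warp is a warp trigger that moves the player to a target location on overlap.
; On BeginPlay it caches the first actor tagged "WarpTarget" as the shared destination.
; When a BP_Player overlaps it, it attaches a teleport particle effect to the player's mesh and moves the player to the target without sweeping.
; It then resets the controller's rotation to face world +X, regardless of the target's orientation.
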(event EventBeginPlay
  (bind _outactors (Actor|GetAllActorswithTag "WarpTarget"))
  (Variables|Default|SetWarpTarget (Utilities|Array|Get(acopy) _outactors)))

(event Collision|EventActorBeginOverlap
  (params (OtherActor :type Actor%20Object%20Reference))
  (bind _asbp_player (Utilities|Casting|CastToBP_Player OtherActor))
  (Effects|SpawnEmitterAttached "/Game/InfinityBladeEffects/Effects/FX_Archive/P_Teleport_Target.P_Teleport_Target" (Variables|/Script/Engine.Character|GetMesh _asbp_player) "None" "0, 0, 0" "0,270.000000, 0")
  (Transformation|SetActorLocation _asbp_player (Transformation|GetActorLocation (Variables|Default|GetWarpTarget)) false false)
  (Pawn|SetControlRotation (Game|GetInstigatorController _asbp_player) (Math|Conversions|RotationFromXVector (Math|Vector|MakeVector 1.0 0.0 0.0))))

(fn ConstructionScript)