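; Blueprint function library of static helpers for sound playback and player stats such as score, health, potions and death checks.
; The sound helper spawns a sound at a given actor's location with a shared attenuation asset, if that actor is valid.
; The stat helpers cast player character 0 to BP_Player and work through its PlayerState, either calling its functions or resetting health to maximum.
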(fn PlaySoundStatic
  (params (Sound :type Sound%20Base%20Object%20Reference) (LocationActor :type Actor%20Object%20Reference))
  (Utilities|IsValid LocationActor
    (:Is%20Valid
      (Audio|SpawnSoundatLocation (LocalVariables|Get__WorldContext) Sound (Transformation|GetActorLocation LocationActor) "0, 0, 0" 1.0 1.0 0.0 "/Game/Sounds/SA_Att.SA_Att" 0))))

(fn AddScore
  (params (Score :type Integer))
  (bind _asbp_player (Utilities|Casting|CastToBP_Player (Game|GetPlayerCharacter 0)))
  (Default|AddScore (Default|GetPlayerState _asbp_player) Score))

(fn UsePostion
  (bind _asbp_player (Utilities|Casting|CastToBP_Player (Game|GetPlayerCharacter 0)))
  (Default|UsePotion (Default|GetPlayerState _asbp_player)))

(fn IncreaseHealth
  (params (Amount :type Float%20%28single-precision%29))
  (bind _asbp_player (Utilities|Casting|CastToBP_Player (Game|GetPlayerCharacter 0)))
  (Default|IncreaseHealth (Default|GetPlayerState _asbp_player) Amount))

(fn DecreaseHealth
  (params (Amount :type Float%20%28single-precision%29))
  (bind _asbp_player (Utilities|Casting|CastToBP_Player (Game|GetPlayerCharacter 0)))
  (Default|DecreaseHealth (Default|GetPlayerState _asbp_player) Amount))

(fn InitialHealth
  (bind _asbp_player (Utilities|Casting|CastToBP_Player (Game|GetPlayerCharacter 0)))
  (Variables|/Game/Player/BP_PlayerState.BP_PlayerState_C|SetMyHealth (Default|GetPlayerState _asbp_player) (Variables|/Game/Player/BP_PlayerState.BP_PlayerState_C|GetMyMaxHealth (Default|GetPlayerState _asbp_player))))

(fn IsPlayerDead
  (bind _asbp_player (Utilities|Casting|CastToBP_Player (Game|GetPlayerCharacter 0)))
  (return (Default|IsDead (Default|GetPlayerState _asbp_player))))