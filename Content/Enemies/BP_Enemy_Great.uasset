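; BP_Enemy_Great is a greatsword enemy that extends a parent enemy Blueprint with its own attack, hit and death montages.
; Attack randomly picks a basic swing or a faster-played, higher-damage skill montage.
; OnCollision and OffCollision toggle the sword collider, whose pawn overlaps apply damage once per actor through the Hitted0 list, cleared on OffCollision.
; SkillEffect spawns an impact particle ahead at ground level with a sound.
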(event OnComponentBeginOverlap(GreatSwordCollision)
  (params (OverlappedComponent :type Primitive%20Component%20Object%20Reference) (OtherActor :type Actor%20Object%20Reference) (OtherComp :type Primitive%20Component%20Object%20Reference) (OtherBodyIndex :type Integer) (bFromSweep :type Boolean) (SweepResult :type Hit%20Result%20Structure%20%28by%20ref%29))
  ;[1 1 1] 충돌 시 대미지 주기
  (if (Utilities|Enum|Equal(Enum) (Collision|GetCollisionObjectType OtherComp) "ECC_Pawn")
    (CallFunction|Damageto 0 (Utilities|Select :Index (Variables|Default|GetAttackSyle) :Option%200 1e+01 :Option%201 45.0) OtherActor)))

(event EventBeginPlay
  ;[1 1 1] 비긴
  (|CallParentFunction)
  (Collision|SetCollisionEnabled (Variables|Default|GetGreatSwordCollision) "NoCollision"))

(event EventTick
  (params (DeltaSeconds :type Float%20%28single-precision%29))
  ;[1 1 1] 띄운 후 체크
  (|CallParentFunction DeltaSeconds))

(event EventPlayHitMontage
  ;[1 1 1] 피격 시
  (|CallParentFunction)
  (Animation|PlayAnimMontage "/Game/Frank_Slash_Pack/Frank_RPG_GreatSword/Animations/IP+RM/GS_Hit.GS_Hit" 1.0 "None"))

(event EventAttack
  ;[1 1 1] 공격 2가지
  (|CallParentFunction)
  (if (not (CallFunction|IsDead))
    (if (not (Variables|Default|GetbAttacking))
      (Variables|Default|SetbAttacking true)
      (bind _output_get (Variables|Default|SetAttackSyle (Math|Random|RandomInteger 2)))
      (switch int _output_get
        (:0
          (Animation|PlayAnimMontage "/Game/Frank_Slash_Pack/Frank_RPG_GreatSword/Animations/IP+RM/GS_Attack.GS_Attack" 1.0 "None"))
        (:1
          (Animation|PlayAnimMontage "/Game/Frank_Slash_Pack/Frank_RPG_GreatSword/Animations/IP+RM/GS_Skill.GS_Skill" 1.5 "None"))))))

(event EventOnCollision
  ;[1 1 1] 충돌체 켜고 끄기
  (|CallParentFunction)
  (Collision|SetCollisionEnabled (Variables|Default|GetGreatSwordCollision) "QueryAndPhysics"))

(event EventOffCollision
  ;[1 1 1] 충돌체 켜고 끄기
  (|CallParentFunction)
  (Collision|SetCollisionEnabled (Variables|Default|GetGreatSwordCollision) "NoCollision")
  (Utilities|Array|Clear (Variables|Default|GetHitted_0)))

(event EventSkillEffect
  ;[1 1 1] 스킬 이펙트
  (|CallParentFunction)
  (Effects|SpawnEmitteratLocation "/Game/InfinityBladeEffects/Effects/FX_Monsters/FX_Monster_Troll/Impact/P_TrollSwingImpact.P_TrollSwingImpact" (- (+ (Transformation|GetActorLocation) (* (Transformation|GetActorForwardVector) 250)) "0, 0,88.000000"))
  (CallFunction|PlaySoundStatic "/Game/Sounds/psahit00_Cue.psahit00_Cue" self))

(event EventDead
  ;[1 1 1] 피격 시
  (|CallParentFunction)
  (Animation|PlayAnimMontage "/Game/Frank_Slash_Pack/Frank_RPG_GreatSword/Animations/IP+RM/GS_DEad.GS_Dead" 1.0 "None"))

(fn ConstructionScript
  (|CallParentFunction))

(fn Damageto
  (params (DamageType :type Damage%20Type%20Class%20Reference) (InDamage :type Float%20%28single-precision%29) (OtherActor :type Actor%20Object%20Reference))
  (if (!= self OtherActor)
    (LocalVariables|SetPrev (Utilities|Array|Length (Variables|Default|GetHitted_0)))
    (Utilities|Array|AddUnique (Variables|Default|GetHitted_0) OtherActor)
    (if (< (LocalVariables|GetPrev) (Utilities|Array|Length (Variables|Default|GetHitted_0)))
      (Game|Damage|ApplyDamage OtherActor InDamage 0 self DamageType))))