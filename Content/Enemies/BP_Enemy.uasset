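; Base enemy Blueprint that handles health, hit reactions and death, leaving attack, montage, skill and collision events empty as virtual hooks for children.
; Point damage drives hit or grabbed state, health loss and death, using damage type classes to select grab or floating launch.
; The player's ground and air combo-finisher flags add directional knockback.
; Tick maintains the grabbed state and capsule-traces falling enemies to restore walking on landing.
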(event Custom|PlayHitMontage
  ;[1 1 1] 가상함수들
)

(event Custom|OnTakePointDamage_Event_0
  (params (DamagedActor :type Actor%20Object%20Reference) (Damage :type Float%20%28single-precision%29) (InstigatedBy :type Controller%20Object%20Reference) (HitLocation :type Vector) (FHitComponent :type Primitive%20Component%20Object%20Reference) (BoneName :type Name) (ShotFromDirection :type Vector) (DamageType :type Damage%20Type%20Object%20Reference) (DamageCauser :type Actor%20Object%20Reference))
  ;[1 1 1] 대미지 이벤트 바인딩
  (Variables|Default|SetDamageType DamageType)
  (Variables|Default|SetDamage Damage)
  (Variables|Default|SetCauser DamageCauser)
  (CallFunction|OffCollision)
  (Utilities|FlowControl|Sequence
    (:then_0
      (CallFunction|PlayHitMontage))
    (:then_1
      (CallFunction|DamageEffect))
    (:then_2
      (Utilities|Casting|CastToGrab (Variables|Default|GetDamageType)
        (:then
          (Variables|Default|SetbGrabbed true)
          (Variables|Default|SetbHitted false))
        (:CastFailed
          (Variables|Default|SetbHitted true)
          (Variables|Default|SetbGrabbed false))))
    (:then_3
      (CallFunction|DecreaseHealth)
      (if (CallFunction|IsDead)
        (CallFunction|Dead)))))

(event Custom|Dead
  ;[1 1 1] 가상함수들
  (Collision|SetCollisionProfileName (Variables|Collision|GetCapsuleComponent) "Spectator" true :!class /Script/Engine.PrimitiveComponent)
  (CallFunction|OffCollision))

(event Custom|DamageEffect
  (bind _returnvalue (Transformation|GetActorRotation))
  (bind _returnvalue_2 (Transformation|GetActorLocation))
  (bind _player (Variables|Default|GetPlayer))
  (bind _returnvalue_3 (Transformation|GetActorLocation _player))
  (bind _returnvalue_4 (Math|Vector|GetUnitDirection(Vector) _returnvalue_3 _returnvalue_2))
  (bind _returnvalue_5 (* _returnvalue_4 1500))
  (Utilities|FlowControl|Sequence
    (:then_0
      (Utilities|Casting|CastToFloating (Variables|Default|GetDamageType))
      (Components|Movement|StopMovementImmediately (Variables|Character|GetCharacterMovement))
      ;[1 1 1] 띄우기
      (if (AI|Components|NavMovement|IsFalling (Variables|Character|GetCharacterMovement))
        (Character|LaunchCharacter "0, 0,200.000000" false false)
        (else
          (Character|LaunchCharacter "0, 0,800.000000" false false)
          (Transformation|SetActorRotation (Math|Rotator|MakeRotator (.roll _returnvalue) 45.0 (.yaw _returnvalue)))
          (Pawn|Components|CharacterMovement|SetMovementMode (Variables|Character|GetCharacterMovement) "MOVE_Flying" 0))))
    (:then_1
      ;[1 1 1] 막타 날리기
      (if (Variables|/Game/Player/BP_Player.BP_Player_C|GetbGourndLast (Variables|Default|GetPlayer))
        (Character|LaunchCharacter (* (Math|Vector|GetUnitDirection(Vector) (Transformation|GetActorLocation (Variables|Default|GetPlayer)) (Transformation|GetActorLocation)) 4000) false false))
      (if (Variables|/Game/Player/BP_Player.BP_Player_C|GetbAirLast (Variables|Default|GetPlayer))
        (Character|LaunchCharacter (Math|Vector|MakeVector (.x _returnvalue_5) (.y _returnvalue_5) -1e+03) false true)))))

(event Custom|Attack
  ;[1 1 1] 가상함수들
)

(event Custom|EndAttack
  ;[1 1 1] 가상함수들
  (Variables|Default|SetbAttacking false))

(event Custom|OnCollision
  ;[1 1 1] 가상함수들
)

(event Custom|OffCollision
  ;[1 1 1] 가상함수들
)

(event Custom|Hitted
  ;[1 1 1] 가상함수들
  (Variables|Default|SetbHitted false)
  (Variables|Default|SetbGrabbed false)
  (Variables|Default|SetbAttacking false))

(event Custom|SkillEffect
  ;[1 1 1] 가상함수들
)

(event Custom|DecreaseHealth
  ;[1 1 1] 가상함수들
  (Variables|Default|SetCurrentHealth (- (Variables|Default|GetCurrentHealth) (Variables|Default|GetDamage))))

(event EventBeginPlay
  ;[1 1 1] 대미지 이벤트 바인딩
  (EventDispatchers|AssignOnTakePointDamage (delegate Custom|OnTakePointDamage_Event_0))
  (bind _asbp_player (Utilities|Casting|CastToBP_Player (Game|GetPlayerCharacter 0)))
  (Variables|Default|SetPlayer _asbp_player)
  (Variables|Default|SetCurrentHealth (Variables|Default|GetMaxHealth)))

(event EventTick
  (params (DeltaSeconds :type Float%20%28single-precision%29))
  (bind _returnvalue (Transformation|GetActorRotation))
  (bind _returnvalue_2 (Transformation|GetActorLocation))
  (Utilities|FlowControl|Sequence
    (:then_0
      ;[1 1 1] 블랙보드에서 "잡힌 상태" 유지하기
      (Utilities|Casting|CastToGrab (Variables|Default|GetDamageType))
      (Variables|Default|SetbGrabbed true)
      (Variables|Default|SetbHitted false))
    (:then_1
      ;[1 1 1] 공콤 맞고 착지 후
      (if (AI|Components|NavMovement|IsFalling (Variables|Character|GetCharacterMovement))
        (Variables|Default|SetbHitted true)
        (Utilities|FlowControl|Delay 0.2)
        (bind _returnvalue_3 (Collision|CapsuleTraceByChannel _returnvalue_2 (+ _returnvalue_2 "0, 0,-44.000000") 44.0 88.0 "TraceTypeQuery1" false 0 "ForOneFrame"))
        (if _returnvalue_3
          (Pawn|Components|CharacterMovement|SetMovementMode (Variables|Character|GetCharacterMovement) "MOVE_Walking" 0)
          (Transformation|SetActorRotation (Math|Rotator|MakeRotator (.roll _returnvalue) 0.0 (.yaw _returnvalue)))
          (Variables|Default|SetbHitted false))))))

(fn ConstructionScript)

(fn IsDead
  (return (<= (Variables|Default|GetCurrentHealth) 0.0)))