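; BP_Wall is a wall actor that builds a spline along a projectile arc from the player character to its Box component.
; MakeSplinePath computes an arcing launch velocity toward the Box, then feeds it into a debug-drawn path prediction against WorldDynamic objects, ignoring the player.
; The spline is cleared on each call and refilled with the predicted positions only when the prediction registers a hit.
; Nothing in this Blueprint calls the event.
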(event Custom|MakeSplinePath
  (bind _returnvalue (Game|GetPlayerCharacter 0))
  (bind _returnvalue_2 (Transformation|GetActorLocation _returnvalue))
  (Utilities|Array|Clear (Variables|Default|GetSplineLocations))
  (Spline|ClearSplinePoints (Variables|Default|GetSpline) true)
  (bind _outlaunchvelocity (Game|SuggestProjectileVelocityCustomArc _returnvalue_2 (Transformation|GetWorldLocation (Variables|Default|GetBox)) 0.0 0.5))
  (bind (_outhit _outpathpositions _outlasttracedestination _returnvalue_3) (Class|GameplayStatics|BlueprintPredictProjectilePathbyObjectType _returnvalue_2 _outlaunchvelocity true 1e+01 (Utilities|Array|MakeArray "ObjectTypeQuery2") false (Utilities|Array|MakeArray (Game|GetPlayerCharacter 0)) "ForDuration" 1.0))
  (if _returnvalue_3
    (bind _output_get (Variables|Default|SetSplineLocations _outpathpositions))
    (Spline|SetSplinePoints (Variables|Default|GetSpline) _output_get "World" true)))

(event EventBeginPlay)

(event Collision|EventActorBeginOverlap
  (params (OtherActor :type Actor%20Object%20Reference)))

(event EventTick
  (params (DeltaSeconds :type Float%20%28single-precision%29)))

(fn ConstructionScript)