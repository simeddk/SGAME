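; BP_GrapplePoint is a grapple point that tracks a target player and shows its current state through an emissive color.
; Setting the target updates the state according to whether that player is valid, and CheckState fires OnGrapplePointStateChanged only when the state differs.
; The construction script creates a dynamic material on the pipe mesh, which state updates tint green, yellow or red.
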(event EventSetGrapplePointTarget
  (params (Player :type BP%20Player%20Object%20Reference))
  (bind _output_get (Variables|Default|SetTargetActor Player))
  (Utilities|IsValid _output_get
    (:Is%20Valid
      (CallFunction|UpdateGrapplePointState "NewEnumerator0"))
    (:Is%20Not%20Valid
      (CallFunction|UpdateGrapplePointState "NewEnumerator2"))))

(event EventUpdateGrapplePointState
  (params (NewState :type EGrappleStateType%20Enum :default "NewEnumerator0"))
  (CallFunction|CheckState NewState)
  (if (Utilities|Enum|Equal(Enum) (Variables|Default|GetGrapplePointState) "NewEnumerator3")
    (Rendering|Material|SetVectorParameterValue (Variables|Default|GetDynamicMAT) "Emissive" "(R=0.000000,G=20.000000,B=0.000000,A=1.000000)" :!class /Script/Engine.MaterialInstanceDynamic)
    (elif (Utilities|Enum|Equal(Enum) (Variables|Default|GetGrapplePointState) "NewEnumerator1")
      (Rendering|Material|SetVectorParameterValue (Variables|Default|GetDynamicMAT) "Emissive" "(R=20.000000,G=20.000000,B=0.000000,A=1.000000)" :!class /Script/Engine.MaterialInstanceDynamic)
      (else
        (Rendering|Material|SetVectorParameterValue (Variables|Default|GetDynamicMAT) "Emissive" "(R=20.000000,G=0.000000,B=0.000000,A=1.000000)" :!class /Script/Engine.MaterialInstanceDynamic)))))

(fn ConstructionScript
  (bind _returnvalue (Rendering|Material|CreateDynamicMaterialInstance (Rendering|Material|GetMaterial (Variables|Default|GetSM_Slums_Pipe_04b) 1) "None" :!class /Script/Engine.KismetMaterialLibrary))
  (bind _output_get (Variables|Default|SetDynamicMAT _returnvalue))
  (Rendering|Material|SetMaterial (Variables|Default|GetSM_Slums_Pipe_04b) 1 _output_get))

(fn CheckState
  (params (NewState :type EGrappleStateType%20Enum :default "NewEnumerator0"))
  (LocalVariables|SetPrevState (Variables|Default|GetGrapplePointState))
  (if (!= NewState (LocalVariables|GetPrevState))
    (Variables|Default|SetGrapplePointState NewState)
    (Default|CallOnGrapplePointStateChanged self (Variables|Default|GetGrapplePointState))
    (else
      (Variables|Default|SetGrapplePointState (LocalVariables|GetPrevState)))))

(fn GetGrapplePointState
  (return (Variables|Default|GetGrapplePointState)))