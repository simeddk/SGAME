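; BP_Cannon is a trap actor that fires projectiles while the player is within range.
; A looping timer started on BeginPlay checks the first player character's distance every second.
; When in range, it spawns a BP_Projectile at each static mesh component tagged "Cannon" and plays a firing sound for each.
; Projectiles take the actor's rotation, so all barrels shoot along its facing without aiming at the player.
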(event Custom|OnTime
  (if (<= (Transformation|GetDistanceTo (Game|GetPlayerCharacter 0) self) 2.5e+03)
    (for _array_element (Actor|GetComponentsbyTag "/Script/Engine.StaticMeshComponent" "Cannon")
      (Game|SpawnActorfromClass "/Game/Trap/BP_Projectile.BP_Projectile_C" (Math|Transform|MakeTransform (Transformation|GetWorldLocation _array_element) (Transformation|GetActorRotation)) "Undefined" self 0)
      (CallFunction|PlaySoundStatic "/Game/Sounds/ttafir00_Cue.ttafir00_Cue" self))))

(event EventBeginPlay
  (Utilities|Time|SetTimerbyEvent (delegate Custom|OnTime) 1.0 true))

(fn ConstructionScript)