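; BP_FlipFlip_Trap is a trap actor that blinks on and off and damages characters that touch it.
; A looping one-second timer drives a FlipFlop that alternately disables the Box collision and hides its ten sprites, then restores both.
; Any Character beginning overlap with the actor takes Trap-type damage, with a shock impact particle at the character and a sound played.
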(event Custom|Timer
  (Utilities|FlowControl|FlipFlop
    (:A
      (Collision|SetCollisionEnabled (Variables|Default|GetBox) "NoCollision")
      (Rendering|SetVisibility (Variables|Default|GetSprite5) false false))
    (:B
      (Collision|SetCollisionEnabled (Variables|Default|GetBox) "QueryAndPhysics")
      (Rendering|SetVisibility (Variables|Default|GetSprite5) true false))))

(event EventBeginPlay
  (Utilities|Time|SetTimerbyEvent (delegate Custom|Timer) 1.0 true))

(event Collision|EventActorBeginOverlap
  (params (OtherActor :type Actor%20Object%20Reference))
  (Utilities|Casting|CastToCharacter OtherActor)
  (if (!= OtherActor self)
    (Game|Damage|ApplyDamage OtherActor 1e+01 0 0 "/Game/Player/Trap.Trap_C")
    (Effects|SpawnEmitteratLocation "/Game/InfinityBladeEffects/Effects/FX_Skill_TeleCharge/P_Skill_Telecharge_Shock_Impact_02.P_Skill_Telecharge_Shock_Impact_02" (Transformation|GetActorLocation OtherActor))
    (CallFunction|PlaySoundStatic "/Game/Sounds/tscfir00.tscfir00" self)))

(fn ConstructionScript)