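; BP_KillZone is a trap volume, apparently for falls, that hurts characters entering its Box.
; On overlap, KillType selects enemies, players or both, and applies Trap point damage.
; Enemies take the Damage variable, while players take a fixed hardcoded amount.
; A player who is still alive then teleports to the game mode's LastCheckPoint with an on-screen message.
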(event OnComponentBeginOverlap(Box)
  (params (OverlappedComponent :type Primitive%20Component%20Object%20Reference) (OtherActor :type Actor%20Object%20Reference) (OtherComp :type Primitive%20Component%20Object%20Reference) (OtherBodyIndex :type Integer) (bFromSweep :type Boolean) (SweepResult :type Hit%20Result%20Structure%20%28by%20ref%29))
  (Variables|Default|SetOtherActor OtherActor)
  (Variables|Default|SetSweepResult SweepResult)
  (switch Utilities|FlowControl|Switch|SwitchonEKillType (Variables|Default|GetKillType)
    (:NewEnumerator2
      (bind _asbp_enemy (Utilities|Casting|CastToBP_Enemy (Variables|Default|GetOtherActor)))
      (Game|Damage|ApplyPointDamage _asbp_enemy (Variables|Default|GetDamage) (Transformation|GetActorLocation (Variables|Default|GetOtherActor)) (Variables|Default|GetSweepResult) 0 self "/Game/Player/Trap.Trap_C"))
    (:NewEnumerator1
      (bind _asbp_player (Utilities|Casting|CastToBP_Player (Variables|Default|GetOtherActor) :!label _label))
      (bind _output_get (Variables|Default|SetPlayer _asbp_player))
      (Game|Damage|ApplyPointDamage _output_get 2e+01 (Transformation|GetActorLocation (Variables|Default|GetOtherActor)) (Variables|Default|GetSweepResult) 0 self "/Game/Player/Trap.Trap_C")
      (bind _player (Variables|Default|GetPlayer)
        (:then
          (Utilities|IsValid (Default|GetPlayerState _player)
            (:Is%20Valid
              (if (not (Default|IsDead (Default|GetPlayerState _player)))
                (bind _asgame_game_mode (Utilities|Casting|CastToGameGameMode (Game|GetGameMode)))
                (bind _lastcheckpoint (Variables|/Game/Game/GameGameMode.GameGameMode_C|GetLastCheckPoint _asgame_game_mode)
                  (:then
                    (Transformation|SetActorLocation (Variables|Default|GetPlayer) (Transformation|GetActorLocation _lastcheckpoint) false false)
                    (Development|PrintString "낙사 전 마지막 체크포인트로 돌아 왔습니다."))
                  (:else))))))
        (:else)))
    (:NewEnumerator3
      (bind _ascharacter (Utilities|Casting|CastToCharacter (Variables|Default|GetOtherActor)))
      (bind _asbp_enemy_2 (Utilities|Casting|CastToBP_Enemy _ascharacter)
        (:then
          (Game|Damage|ApplyPointDamage _asbp_enemy_2 (Variables|Default|GetDamage) (Transformation|GetActorLocation (Variables|Default|GetOtherActor)) (Variables|Default|GetSweepResult) 0 self "/Game/Player/Trap.Trap_C"))
        (:CastFailed
          (goto _label))))))

(fn ConstructionScript)