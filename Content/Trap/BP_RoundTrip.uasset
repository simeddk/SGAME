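; BP_RoundTrip is a trap actor that moves back and forth between its placed location and a relative target offset.
; BeginPlay stores both endpoints in world space, adding RelativeTargetLocation as an unrotated world-axis offset.
; Tick moves the actor toward the target at Speed scaled by delta time, without sweeping.
; It swaps endpoints once distance from the start reaches the path length, without snapping away any overshoot.
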(event EventBeginPlay
  (bind _returnvalue (Transformation|GetActorLocation))
  (Variables|Default|SetGlobalStartLocation _returnvalue)
  (Variables|Default|SetGlobalTargetLocation (+ _returnvalue (Variables|Default|GetRelativeTargetLocation))))

(event EventTick
  (params (DeltaSeconds :type Float%20%28single-precision%29))
  (Variables|Default|SetTotalDistance (Math|Vector|VectorLength (- (Variables|Default|GetGlobalTargetLocation) (Variables|Default|GetGlobalStartLocation)))) ; 가야할 거리
  (Variables|Default|SetCurrentDistance (Math|Vector|VectorLength (- (Transformation|GetActorLocation) (Variables|Default|GetGlobalStartLocation)))) ; 시작점으로부터 점점 멀어진 거리
  (if (>= (Variables|Default|GetCurrentDistance) (Variables|Default|GetTotalDistance)) ; 점점 멀어져서 가야할 거리에 도달하면
    (Variables|Default|SetTemp (Variables|Default|GetGlobalStartLocation))
    (Variables|Default|SetGlobalStartLocation (Variables|Default|GetGlobalTargetLocation))
    (Variables|Default|SetGlobalTargetLocation (Variables|Default|GetTemp)))
  (Transformation|SetActorLocation (+ (* (* (Math|Vector|Normalize (- (Variables|Default|GetGlobalTargetLocation) (Variables|Default|GetGlobalStartLocation))) (Utilities|Time|GetWorldDeltaSeconds)) (Variables|Default|GetSpeed)) (Transformation|GetActorLocation)) false false))

(fn ConstructionScript)