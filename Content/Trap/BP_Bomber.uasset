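; BP_Bomber is a one-shot trap that homes in on the player and explodes.
; Box overlap by BP_Player turns the billboard's dynamic material emissive red, ignites sparks and plays a sound.
; A timeline lerps only the Sphere from its start toward the player's live location.
; After a short delay, Sphere collision switches on to apply Trap damage on overlap, explosion effects play, and the actor destroys itself.
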(event OnComponentBeginOverlap(Box)
  (params (OverlappedComponent :type Primitive%20Component%20Object%20Reference) (OtherActor :type Actor%20Object%20Reference) (OtherComp :type Primitive%20Component%20Object%20Reference) (OtherBodyIndex :type Integer) (bFromSweep :type Boolean) (SweepResult :type Hit%20Result%20Structure%20%28by%20ref%29))
  (bind _asbp_player (Utilities|Casting|CastToBP_Player OtherActor))
  (Utilities|FlowControl|DoOnce false
    (:Completed
      (CallFunction|PlaySoundStatic "/Game/Sounds/laserb_Cue.laserb_Cue" _asbp_player)
      (Rendering|Material|SetVectorParameterValue (Variables|Default|GetDynamicMat) "Emissive" "(R=20.000000,G=0.000000,B=0.000000,A=1.000000)" :!class /Script/Engine.MaterialInstanceDynamic)
      (Effects|SpawnEmitterAttached "/Game/InfinityBladeEffects/Effects/FX_Monsters/FX_Monster_Gruntling/Bomber/P_BomberSparks_Ignite.P_BomberSparks_Ignite" (Variables|Default|GetSphere) "" "0, 0, 0" "0, 0, 0" "2.000000,2.000000,2.000000")
      (Utilities|IsValid OtherActor
        (:Is%20Valid
          (bind _out (Timeline|타임라인_0 Play)
            (:Update
              (Transformation|SetWorldLocation (Variables|Default|GetSphere) (Math|Vector|Lerp(Vector) (Variables|Default|GetStart) (Transformation|GetActorLocation OtherActor) _out) false false)
              (Variables|Default|SetTarget (Math|Vector|Lerp(Vector) (Variables|Default|GetStart) (Transformation|GetActorLocation OtherActor) _out)))
            (:Finished
              (Utilities|FlowControl|Delay 0.25)
              (Collision|SetCollisionEnabled (Variables|Default|GetSphere) "QueryAndPhysics")
              (Effects|SpawnEmitteratLocation "/Game/Explosions/Particles/P_ImpactExplosion.P_ImpactExplosion" (Variables|Default|GetTarget))
              (CallFunction|PlaySoundStatic "/Game/Sounds/psahit00_Cue.psahit00_Cue" self)
              (Utilities|FlowControl|Delay 0.2)
              (Actor|DestroyActor))))))))

(event OnComponentBeginOverlap(Sphere)
  (params (OverlappedComponent :type Primitive%20Component%20Object%20Reference) (OtherActor :type Actor%20Object%20Reference) (OtherComp :type Primitive%20Component%20Object%20Reference) (OtherBodyIndex :type Integer) (bFromSweep :type Boolean) (SweepResult :type Hit%20Result%20Structure%20%28by%20ref%29))
  (Game|Damage|ApplyDamage OtherActor 15.0 0 self "/Game/Player/Trap.Trap_C")
  (Actor|DestroyActor))

(event EventBeginPlay
  (Collision|SetCollisionEnabled (Variables|Default|GetSphere) "NoCollision")
  (Variables|Default|SetStart (Transformation|GetActorLocation)))

(fn ConstructionScript
  (bind _returnvalue (Rendering|Material|CreateDynamicMaterialInstance (Rendering|Material|GetMaterial (Variables|Default|GetMaterialBillboard) 0) "None" :!class /Script/Engine.KismetMaterialLibrary))
  (bind _output_get (Variables|Default|SetDynamicMat _returnvalue))
  (Rendering|Material|SetMaterial (Variables|Default|GetMaterialBillboard) 0 _output_get))