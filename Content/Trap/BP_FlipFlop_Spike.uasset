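; BP_FlipFlop_Spike is a trap whose spikes cycle continuously and damage BP_Player when it begins overlapping the actor.
; After a start delay, a FlipFlop alternates playing a timeline forward and reversing it from the end with a sound cue, re-triggered on each Finished.
; Timeline updates set the relative Z of every static mesh component tagged "Spike".
; Overlap applies Trap-type damage regardless of spike position.
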(event EventBeginPlay
  (Utilities|FlowControl|Delay (Variables|Default|GetStart))
  (Utilities|FlowControl|FlipFlop :!label _label
    (:A
      (Components|Timeline|SetPlayRate (Variables|Default|GetTimeline) (Variables|Default|GetPlayRate))
      (bind _out (Timeline|Timeline Play)
        (:Update
          (for _array_element (Actor|GetComponentsbyTag "/Script/Engine.StaticMeshComponent" "Spike")
            (Transformation|SetRelativeLocation _array_element (Math|Vector|MakeVector (.x (Variables|/Script/Engine.SceneComponent|GetRelativeLocation _array_element)) (.y (Variables|/Script/Engine.SceneComponent|GetRelativeLocation _array_element)) _out) false false)))
        (:Finished
          (goto _label))))
    (:B
      (CallFunction|PlaySoundStatic "/Game/Sounds/Spike_Cue.Spike_Cue" self)
      (Timeline|Timeline ReverseFromEnd))))

(event Collision|EventActorBeginOverlap
  (params (OtherActor :type Actor%20Object%20Reference))
  (bind _asbp_player (Utilities|Casting|CastToBP_Player OtherActor))
  (Game|Damage|ApplyDamage _asbp_player 1e+01 0 0 "/Game/Player/Trap.Trap_C"))

(fn ConstructionScript)