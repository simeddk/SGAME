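; BP_PlayerState is the player state that holds a player's score, health and potion count.
; Helper functions add score, clamp health changes and consume a potion to heal with a sound and particle effect while alive.
; RepNotify handlers push changes to the widget on the BP_Player cached at BeginPlay through the owning controller, animating it when score changes.
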(event EventBeginPlay
  (bind _ascontroller (Utilities|Casting|CastToController (Components|GetOwner)))
  (bind _asbp_player (Utilities|Casting|CastToBP_Player (Pawn|GetControlledPawn _ascontroller)))
  (Variables|Default|SetPlayer _asbp_player))

(event EventTick
  (params (DeltaSeconds :type Float%20%28single-precision%29)))

(fn ConstructionScript)

(fn OnRepMyScore
  (bind _player (Variables|Default|GetPlayer))
  (bind _widget (Variables|/Game/Player/BP_Player.BP_Player_C|GetWidget _player))
  (Default|SetScore _widget)
  (Class|UserWidget|PlayAnimationForward _widget (Variables|/Game/Widgets/WB_Player.WB_Player_C|GetAnim _widget) 1.0 false))

(fn AddScore
  (params (Score :type Integer))
  (Variables|Default|SetMyScore (+ (Variables|Default|GetMyScore) Score)))

(fn OnRepMyHealth
  (Default|UpdateHealth (Variables|/Game/Player/BP_Player.BP_Player_C|GetWidget (Variables|Default|GetPlayer)) (Variables|Default|GetMyHealth) (Variables|Default|GetMyMaxHealth)))

(fn OnRepMyPotionCount
  (Default|SetPotionCount (Variables|/Game/Player/BP_Player.BP_Player_C|GetWidget (Variables|Default|GetPlayer))))

(fn IncreaseHealth
  (params (Amount :type Float%20%28single-precision%29))
  (Variables|Default|SetMyHealth (Math|Float|Clamp(Float) (+ Amount (Variables|Default|GetMyHealth)) 0.0 (Variables|Default|GetMyMaxHealth))))

(fn DecreaseHealth
  (params (Amount :type Float%20%28single-precision%29))
  (Variables|Default|SetMyHealth (Math|Float|Clamp(Float) (- (Variables|Default|GetMyHealth) Amount) 0.0 (Variables|Default|GetMyMaxHealth))))

(fn UsePotion
  (if (and (> (Variables|Default|GetMyPotionCount) 0) (not (CallFunction|IsDead)))
    (CallFunction|IncreaseHealth 5e+01)
    (Variables|Default|SetMyPotionCount (Math|Integer|Clamp(Integer) (- (Variables|Default|GetMyPotionCount) 1) 0 3))
    (CallFunction|PlaySoundStatic "/Game/Sounds/heavy_swallowwav-14682.heavy_swallowwav-14682" (Variables|Default|GetPlayer))
    (Effects|SpawnEmitterAttached "/Game/InfinityBladeEffects/Effects/FX_Ability/Heal/P_Health_Pickup_01.P_Health_Pickup_01" (Variables|/Script/Engine.Character|GetMesh (Variables|Default|GetPlayer)) "None")))

(fn IsDead
  (return (<= (Variables|Default|GetMyHealth) 0.0)))