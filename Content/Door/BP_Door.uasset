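; BP_Door is an automatic sliding double door with a rotating lock that opens when a Character overlaps it and closes when they leave.
; One timeline slides the Left and Right panels apart in opposite directions and rolls the Lock, reversing on exit, with open and close sounds.
; A dynamic material on the Lock turns its emissive green on opening and back to red once the reverse finishes.
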(event EventBeginPlay
  (bind _returnvalue (Rendering|Material|CreateDynamicMaterialInstance "/Game/Door/MAT_Lock.MAT_Lock" "None" :!class /Script/Engine.KismetMaterialLibrary))
  (bind _output_get (Variables|Default|SetLockMaterial _returnvalue))
  (Rendering|Material|SetMaterial (Variables|Default|GetLock) 0 _output_get))

(event Collision|EventActorBeginOverlap
  (params (OtherActor :type Actor%20Object%20Reference))
  (Utilities|Casting|CastToCharacter OtherActor)
  (Rendering|Material|SetVectorParameterValue (Variables|Default|GetLockMaterial) "Emissive" "(R=0.000000,G=20.000000,B=0.000000,A=1.000000)" :!class /Script/Engine.MaterialInstanceDynamic)
  (Audio|PlaySound2D "/Game/Door/Doom-Door-Open_mp3.Doom-Door-Open_mp3" 1.0 1.0 0.2 0 0)
  (bind (_direction _door _lock) (Timeline|Timeline Play)
    (:Update
      (Utilities|FlowControl|Sequence
        (:then_0
          ;[1 1 1] Door Open
          (Transformation|SetRelativeLocation (Variables|Default|GetRight) (Math|Vector|MakeVector 0.0 _door 0.0) false false)
          (Transformation|SetRelativeLocation (Variables|Default|GetLeft) (* (Math|Vector|MakeVector 0.0 _door 0.0) -1) false false))
        (:then_1
          ;[1 1 1] Lock Rotation
          (Transformation|SetRelativeRotation (Variables|Default|GetLock) (Math|Rotator|MakeRotator _lock 0.0 0.0) false false))))
    (:Finished
      ;[1 1 1] Reset LockColor
      (if (Utilities|Enum|Equal(Enum) _direction "Backward")
        (Rendering|Material|SetVectorParameterValue (Variables|Default|GetLockMaterial) "Emissive" "(R=20.000000,G=0.000000,B=0.000000,A=1.000000)" :!class /Script/Engine.MaterialInstanceDynamic)))))

(event Collision|EventActorEndOverlap
  (params (OtherActor :type Actor%20Object%20Reference))
  (Utilities|Casting|CastToCharacter OtherActor)
  (Audio|PlaySound2D "/Game/Door/Doom-Door-Close_mp3.Doom-Door-Close_mp3" 1.0 1.0 0.3 0 0)
  (bind (_direction _door _lock) (Timeline|Timeline Reverse)
    (:Update
      (Utilities|FlowControl|Sequence
        (:then_0
          ;[1 1 1] Door Open
          (Transformation|SetRelativeLocation (Variables|Default|GetRight) (Math|Vector|MakeVector 0.0 _door 0.0) false false)
          (Transformation|SetRelativeLocation (Variables|Default|GetLeft) (* (Math|Vector|MakeVector 0.0 _door 0.0) -1) false false))
        (:then_1
          ;[1 1 1] Lock Rotation
          (Transformation|SetRelativeRotation (Variables|Default|GetLock) (Math|Rotator|MakeRotator _lock 0.0 0.0) false false))))
    (:Finished
      ;[1 1 1] Reset LockColor
      (if (Utilities|Enum|Equal(Enum) _direction "Backward")
        (Rendering|Material|SetVectorParameterValue (Variables|Default|GetLockMaterial) "Emissive" "(R=20.000000,G=0.000000,B=0.000000,A=1.000000)" :!class /Script/Engine.MaterialInstanceDynamic)))))

(fn ConstructionScript)